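; Bomb actor that kills the player on contact and restarts the game on MainMap.
; BeginPlay scales it down to a tenth size, and any overlap calls ExecuteEffect, which acts only on Player1 by destroying it and opening the level.
; Tick accumulates LiveTime and destroys the bomb once it exceeds MaxLiveTime.
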(event `self.ReceiveBeginPlay`
  (`self.SetActorScale3D` (0.1 0.1 0.1)))

(event `self.ReceiveActorBeginOverlap`
  (params (OtherActor :type "Actor Object Reference"))
  (`self.ExecuteEffect ` OtherActor))

(event `self.ReceiveTick`
  (params (DeltaSeconds :type "Float (single-precision)"))
  (set `self.LiveTime` (+ DeltaSeconds (`self.LiveTime`)))
  (`/Engine/EditorBlueprintResources/StandardMacros.CompareFloat` (`self.LiveTime`) (`self.MaxLiveTime`)
    (:`>`
      (if true
        (`self.K2_DestroyActor`)))))

(fn `ExecuteEffect `
  (params (Object :type "Actor Object Reference"))
  (bind _asplayer_1 (cast `/Game/Blueprints/Player1` Object))
  (`self.K2_DestroyActor` _asplayer_1)
  (`GameplayStatics.OpenLevel` "MainMap"))

(fn `UserConstructionScript`)