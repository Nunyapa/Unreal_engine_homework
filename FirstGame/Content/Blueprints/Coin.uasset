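; Coin is a spinning pickup actor that adds one to the player's coin score.
; It shrinks its scale on BeginPlay, rotates every Tick, and accumulates LiveTime to destroy itself once MaxLiveTime is exceeded.
; On overlap, ExecuteEffect casts the other actor to Player1, increments CoinScore and refreshes the collected text, then the coin destroys itself whatever actor touched it.
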(event `self.ReceiveActorBeginOverlap`
  (params (OtherActor :type "Actor Object Reference"))
  (`self.ExecuteEffect` OtherActor)
  (`self.K2_DestroyActor`))

(event `self.ReceiveBeginPlay`
  (`self.SetActorScale3D` (0.1 0.1 0.05)))

(event `self.ReceiveTick`
  (params (DeltaSeconds :type "Float (single-precision)"))
  (`self.K2_AddActorLocalRotation` (* (struct :`Pitch` 180.0 :`Roll` 180.0) DeltaSeconds))
  (set `self.LiveTime` (+ DeltaSeconds (`self.LiveTime`)))
  (`/Engine/EditorBlueprintResources/StandardMacros.CompareFloat` (`self.LiveTime`) (`self.MaxLiveTime`)
    (:`>`
      (if true
        (`self.K2_DestroyActor`)))))

(fn `ExecuteEffect`
  (params (Object :type "Actor Object Reference (by ref)"))
  (bind _asplayer_1 (cast `/Game/Blueprints/Player1` Object))
  (set `/Game/Blueprints/Player1.CoinScore` (+ 1 (`/Game/Blueprints/Player1.CoinScore` _asplayer_1)) _asplayer_1)
  (`/Game/Blueprints/Player1.SetCollectedText` _asplayer_1))

(fn `UserConstructionScript`)