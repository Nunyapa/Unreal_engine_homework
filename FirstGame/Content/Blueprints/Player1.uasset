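; Player pawn for a tunnel-flying game that moves forward at an accelerating speed, scaled by a boost factor, and steers with the mouse.
; BeginPlay creates the HUD and dynamic material, then chains tunnel segments from each last SpawnPoint, adding a randomly offset Slime, Boost, Coin or Bomb.
; Helpers update the coin text, fade the material's TextureAlpha below five coins, and identify Slime, Boost or Coin objects, excluding Bomb.
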(event `self.ReceiveBeginPlay`
  (bind _returnvalue (`PrimitiveComponent.CreateDynamicMaterialInstance` (`self.Player`) 0 "/Game/Materials/PlayerMaterial.PlayerMaterial" "None"))
  (set `self.PlayerMaterial` _returnvalue)
  (`self.SetActorScale3D` (0.05 0.05 0.05))
  (bind _returnvalue_2 (`|GenericCreateObject` "/Game/Blueprints/HUD.HUD_C" self))
  (bind _output_get (set `self.HUDInstance` _returnvalue_2))
  (`UserWidget.AddToViewport` _output_get 0)
  (for _ (range 6)
    (`/Engine/EditorBlueprintResources/StandardMacros.IsValid` (`self.LastSpawnedTunnel`)
      (:`Is Valid`
        (`self.SpawnNextTunnel`))
      (:`Is Not Valid`
        (`self.SpawnTunnel` (0.0 0.0 0.0))))))

(event `self.ReceiveTick`
  (params (DeltaSeconds :type "Float (single-precision)"))
  (bind _returnvalue (`self.ConsumeMovementInputVector`))
  (`SceneComponent.K2_AddLocalOffset` (`self.Player`) (+ (* _returnvalue (* DeltaSeconds (`self.ControlSpeed`))) (* (`self.GetActorForwardVector`) (* DeltaSeconds (`self.BoostEffect`) (`self.Speed`)))) true false)
  (set `self.Speed` (+ (`self.Acceleration`) (`self.Speed`))))

(event `InputAxis|MouseAxisX`
  (params (AxisValue :type "Float (single-precision)"))
  (`self.AddMovementInput` (`self.GetActorRightVector`) AxisValue))

(event `InputAxis|MouseAxisY`
  (params (AxisValue :type "Float (single-precision)"))
  (`self.AddMovementInput` (`self.GetActorUpVector`) AxisValue))

(fn `CastToObstacle`
  (params (Object :type "Actor Object Reference"))
  (returns (IsValid :type Boolean))
  (cast `/Game/Blueprints/Slime` Object
    (:`then`
      _)
    (:`CastFailed`
      (cast `/Game/Blueprints/Boost` Object
        (:`then`
          _)
        (:`CastFailed`
          (cast `/Game/Blueprints/Coin` Object
            (:`then`
              _)
            (:`CastFailed`
              (return false)))))))
  (return true))

(fn `ChangeAlpha`
  (bind _playermaterial (`self.PlayerMaterial`))
  (bind _coinscore (`self.CoinScore`))
  (`/Engine/EditorBlueprintResources/StandardMacros.CompareInt` _coinscore 5
    (:`<`
      (if true
        (`MaterialInstanceDynamic.SetScalarParameterValue` _playermaterial "TextureAlpha" (- 1.0 (/ (`KismetMathLibrary.Conv_IntToDouble` _coinscore) 5.0)))
        (else
          (`MaterialInstanceDynamic.SetScalarParameterValue` _playermaterial "TextureAlpha" 0.0))))))

(fn `SetCollectedText`
  (`TextBlock.SetText` (`/Game/Blueprints/HUD.CollectedText` (`self.HUDInstance`)) (`|FormatText` "Collected coins: {collected}" (`self.CoinScore`)))
  (`self.ChangeAlpha`))

(fn `SpawnNextTunnel`
  (bind _returnvalue (`SceneComponent.K2_GetComponentLocation` (`/Game/Blueprints/Tunnel.SpawnPoint` (`self.LastSpawnedTunnel`))))
  (`self.SpawnTunnel` _returnvalue)
  (`self.SpawnRandomEnemy` _returnvalue))

(fn `SpawnRandomEnemy`
  (params (SpawnLocation :type "Vector Structure"))
  (`|SpawnActorFromClass` (select `int` (`KismetMathLibrary.RandomInteger` 4) :`0` "/Game/Blueprints/Slime.Slime_C" :`1` "/Game/Blueprints/Boost.Boost_C" :`2` "/Game/Blueprints/Coin.Coin_C" :`3` "/Game/Blueprints/Bomb.Bomb_C" :!type "Actor Class Reference") (`KismetMathLibrary.MakeTransform` (+ SpawnLocation (`KismetMathLibrary.MakeVector` 0.0 (`KismetMathLibrary.RandomFloatInRange` -40.0 40.0) (`KismetMathLibrary.RandomFloatInRange` -40.0 40.0))) (struct) (0.2 0.2 0.2)) "Undefined" "OverrideRootScale" null null))

(fn `SpawnTunnel`
  (params (SpawnLocation :type "Vector Structure"))
  (bind _returnvalue (`|SpawnActorFromClass` "/Game/Blueprints/Tunnel.Tunnel_C" (`KismetMathLibrary.MakeTransform` SpawnLocation) "Undefined" "OverrideRootScale" null null))
  (set `self.LastSpawnedTunnel` _returnvalue))

(fn `UserConstructionScript`)