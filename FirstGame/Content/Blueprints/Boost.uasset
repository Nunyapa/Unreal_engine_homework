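; Boost pickup actor that raises a Player1's Speed by a fixed amount when touched.
; Overlap on its Cone hides the actor, calls ExecuteEffect to cast the other actor and add the speed, then destroys the boost, whatever actor touched it.
; Tick accumulates LiveTime and destroys the boost once it exceeds MaxLiveTime.
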(event `self.ReceiveTick`
  (params (DeltaSeconds :type "Float (single-precision)"))
  (set `self.LiveTime` (+ DeltaSeconds (`self.LiveTime`)))
  (`/Engine/EditorBlueprintResources/StandardMacros.CompareFloat` (`self.LiveTime`) (`self.MaxLiveTime`)
    (:`>`
      (if true
        (`self.K2_DestroyActor`)))))

(event `self.Cone.OnComponentBeginOverlap`
  (params (OverlappedComponent :type "PrimitiveComponent Object Reference") (OtherActor :type "Actor Object Reference") (OtherComp :type "PrimitiveComponent Object Reference") (OtherBodyIndex :type Integer) (bFromSweep :type Boolean) (SweepResult :type "HitResult Structure (by ref)"))
  (`self.SetActorHiddenInGame` true)
  (`self.ExecuteEffect` OtherActor)
  (`self.K2_DestroyActor`))

(fn `ExecuteEffect`
  (params (Object :type "Actor Object Reference"))
  (bind _asplayer_1 (cast `/Game/Blueprints/Player1` Object))
  (set `/Game/Blueprints/Player1.Speed` (+ 20.0 (`/Game/Blueprints/Player1.Speed` _asplayer_1)) _asplayer_1))

(fn `UserConstructionScript`)