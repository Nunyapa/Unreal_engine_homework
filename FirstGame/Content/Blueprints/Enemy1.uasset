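; Enemy1 is an enemy actor with a lifetime counter and a speed effect on Player1.
; Tick accumulates LiveTime against MaxLiveTime, but a constant-false branch keeps DestroyActor from running.
; ExecuteEffect casts its Object to Player1, halves Speed, sets a three-second timer naming ExecuteEffect itself, then immediately doubles Speed back, leaving no lasting slowdown.
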(event `self.ReceiveTick`
  (params (DeltaSeconds :type "Float (single-precision)"))
  (set `self.LiveTime` (+ DeltaSeconds (`self.LiveTime`)))
  (`/Engine/EditorBlueprintResources/StandardMacros.CompareFloat` (`self.LiveTime`) (`self.MaxLiveTime`)
    (:`>`
      (if false
        (`self.K2_DestroyActor`)))))

(fn `ExecuteEffect`
  (params (Object :type "Actor Object Reference"))
  (bind _asplayer_1 (cast `/Game/Blueprints/Player1` Object))
  (set `/Game/Blueprints/Player1.Speed` (/ (`/Game/Blueprints/Player1.Speed` _asplayer_1) 2.0) _asplayer_1)
  (`KismetSystemLibrary.K2_SetTimer` "Enemy1" "ExecuteEffect" 3.0)
  (set `/Game/Blueprints/Player1.Speed` (* 2.0 (`/Game/Blueprints/Player1.Speed` _asplayer_1)) _asplayer_1))

(fn `UserConstructionScript`)